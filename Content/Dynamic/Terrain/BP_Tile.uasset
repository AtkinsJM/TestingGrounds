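; BP_Tile is a terrain tile for an endless level, exposing an attach point transform and a one-way barrier.
; The barrier starts non-colliding with a blue tint from a dynamic material instance.
; When the player pawn leaves the barrier volume on its +X side, the barrier turns solid and red.
; The tile then tells InfiniteTerrainGameMode to spawn a tile and destroy an old one.
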(event OnComponentEndOverlap(BarrierVolume)
  (params (OverlappedComponent :type Primitive%20Component%20Object%20Reference) (OtherActor :type Actor%20Object%20Reference) (OtherComp :type Primitive%20Component%20Object%20Reference) (OtherBodyIndex :type Integer))
  (bind _returnvalue (CallFunction|PlayerPassedBarrier OverlappedComponent OtherActor))
  (if _returnvalue
    (CallFunction|ActivateBarrier)
    (bind _asinfinite_terrain_game_mode (Utilities|Casting|CastToInfiniteTerrainGameMode (Game|GetGameMode)))
    (Default|SpawnTile _asinfinite_terrain_game_mode)
    (Default|DestroyOldTile _asinfinite_terrain_game_mode)))

(event EventBeginPlay
  (CallFunction|DeactivateBarrier))

(event Collision|EventActorBeginOverlap
  (params (OtherActor :type Actor%20Object%20Reference)))

(fn ConstructionScript
  (bind _returnvalue (Rendering|Material|CreateDynamicMaterialInstance (Variables|Default|GetBarrier) 0 0 "None" :!class /Script/Engine.PrimitiveComponent))
  (Variables|Default|SetDynamic%20Barrier%20Material _returnvalue))

(fn GetAttachPoint
  (return (Transformation|GetWorldTransform (Variables|Default|GetAttachPoint))))

(fn DeactivateBarrier
  (Collision|SetCollisionEnabled (Variables|Default|GetBarrier) "NoCollision")
  (Rendering|Material|SetVectorParameterValue (Variables|Default|GetDynamic%20Barrier%20Material) "Tint" "(R=0.135668,G=0.415116,B=1.000000,A=1.000000)" :!class /Script/Engine.MaterialInstanceDynamic))

(fn ActivateBarrier
  (Collision|SetCollisionEnabled (Variables|Default|GetBarrier) "QueryAndPhysics")
  (Rendering|Material|SetVectorParameterValue (Variables|Default|GetDynamic%20Barrier%20Material) "Tint" "(R=1.000000,G=0.270759,B=0.280706,A=1.000000)" :!class /Script/Engine.MaterialInstanceDynamic))

(fn PlayerPassedBarrier
  (params (Barrier :type Scene%20Component%20Object%20Reference) (Player :type Actor%20Object%20Reference))
  (return (Math|Boolean|ANDBoolean (< (.x (Transformation|GetWorldLocation Barrier)) (.x (Transformation|GetActorLocation Player))) (== Player (Game|Player|GetPlayerPawn 0)) (not (Class|PrimitiveComponent|IsCollisionEnabled (Variables|Default|GetBarrier))))))