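; AI controller for guard NPCs that starts the GuardBehaviour behavior tree on the PatrolData blackboard at BeginPlay.
; AI perception updates ignore actors tagged Guard.
; A sensed target is written to the blackboard as the focal actor, along with the pawn's current location as the point where it left patrol.
; An unsuccessful stimulus clears only the focal actor, leaving that saved location in place.
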(event OnTargetPerceptionUpdated(AIPerception)
  (params (Actor :type Actor%20Object%20Reference) (Stimulus :type AI%20Stimulus%20Structure))
  (if (not (Actor|ActorHasTag Actor "Guard"))
    (if (.bSuccessfullySensed (Utilities|Struct|BreakAIStimulus Stimulus))
      (AI|Components|Blackboard|SetValueasObject (AI|GetBlackboard 0) (Variables|Default|GetFocalActorKey) Actor)
      (AI|Components|Blackboard|SetValueasVector (AI|GetBlackboard 0) (Variables|Default|GetLeavePatrolLocationKey) (Transformation|GetActorLocation (Pawn|GetControlledPawn)))
      (else
        (AI|Components|Blackboard|ClearValue (AI|GetBlackboard 0) (Variables|Default|GetFocalActorKey))))))

(event EventBeginPlay
  (Class|AIController|UseBlackboard "/Game/Dynamic/Character/AI/PatrolData.PatrolData")
  (AI|RunBehaviorTree "/Game/Dynamic/Character/AI/GuardBehaviour.GuardBehaviour"))

(fn ConstructionScript)