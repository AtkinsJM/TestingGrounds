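; AI controller for guard NPCs that runs the guard behavior tree on the patrol blackboard at BeginPlay.
; On each perception update it stores a sensed actor as the focal actor, or clears it when sensing fails, ignoring actors tagged Guard.
; Every update, including those from guards, also saves the pawn's current location as the leave-patrol location.
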(event OnTargetPerceptionUpdated(AIPerception)
  (params (Actor :type Actor%20Object%20Reference) (Stimulus :type AI%20Stimulus%20Structure))
  ;[1 1 1] On Perception
  (CallFunction|UpdateFocalActorKey Actor Stimulus)
  (CallFunction|UpdateLeavePatrolLocationKey))

(event EventBeginPlay
  ;[1 1 1] BeginPlay
  (Class|AIController|UseBlackboard "/Game/Dynamic/Character/AI/BB_PatrolData.BB_PatrolData")
  (AI|RunBehaviorTree "/Game/Dynamic/Character/AI/BT_GuardBehaviour.BT_GuardBehaviour"))

(fn ConstructionScript)

(fn UpdateFocalActorKey
  (params (Focal%20Actor :type Actor%20Object%20Reference) (AIStimulus :type AI%20Stimulus%20Structure%20%28by%20ref%29))
  (if (not (Actor|ActorHasTag Focal%20Actor "Guard"))
    (if (.bSuccessfullySensed (Utilities|Struct|BreakAIStimulus AIStimulus))
      (AI|Components|Blackboard|SetValueasObject (AI|GetBlackboard 0) (Variables|Default|GetFocalActorKey) Focal%20Actor)
      (else
        (AI|Components|Blackboard|ClearValue (AI|GetBlackboard 0) (Variables|Default|GetFocalActorKey))))))

(fn UpdateLeavePatrolLocationKey
  (AI|Components|Blackboard|SetValueasVector (AI|GetBlackboard 0) (Variables|Default|GetLeavePatrolLocationKey) (Transformation|GetActorLocation (Pawn|GetControlledPawn))))